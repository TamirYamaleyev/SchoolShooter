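; Mana component that tracks a current mana pool, starting it at MaxMana on BeginPlay.
; A looping timer runs RegenManaTick, adding interval-scaled regen with no upper clamp, while RestoreMana clamps to the valid range.
; TryConsumeMana deducts the lesser of truncated mana and cost, allowing partial spends, then returns that minimum recomputed from the reduced mana.
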(event `self.ReceiveBeginPlay`
  (set `self.CurrentMana` (`self.MaxMana`))
  (`KismetSystemLibrary.K2_SetTimer` null "RegenManaTick" (`self.ManaRegenInterval`) true))

(fn `RegenManaTick`
  (set `self.CurrentMana` (+ (* (`self.ManaRegenInterval`) (`self.ManaRegenAmount`)) (`self.CurrentMana`))))

(fn `RestoreMana`
  (params (Amount :type "Float (double-precision)"))
  (set `self.CurrentMana` (`KismetMathLibrary.FClamp` (+ Amount (`self.CurrentMana`)) 0.0 (`self.MaxMana`))))

(fn `TryConsumeMana`
  (params (Cost :type "Float (double-precision)"))
  (returns (AmountConsumed :type "Float (double-precision)"))
  (bind _currentmana (`self.CurrentMana`))
  (bind _returnvalue (`KismetMathLibrary.Min` (`KismetMathLibrary.FTrunc` _currentmana) (`KismetMathLibrary.FTrunc` Cost)))
  (set `self.CurrentMana` (- _currentmana _returnvalue))
  (return (`KismetMathLibrary.Conv_IntToDouble` _returnvalue)))