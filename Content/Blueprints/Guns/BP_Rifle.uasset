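; BP_Rifle is a gun Blueprint that fires projectiles at a limited rate, extending the Shoot event of its parent.
; Shoot calls the parent, then, if CanShoot is set, clears it and spawns a BP_PistolProjectile at the FirePoint transform, ignoring collision.
; A timer of FireRate length then calls ResetShot to re-enable firing.
; The rifle reuses the pistol's projectile class.
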(event `self.Shoot`
  (`parent.Shoot`)
  (if (`self.CanShoot`)
    (set `self.CanShoot` false)
    (`|SpawnActorFromClass` "/Game/Blueprints/Guns/Bullets/BP_PistolProjectile.BP_PistolProjectile_C" (`SceneComponent.K2_GetComponentToWorld` (`self.FirePoint`)) "AlwaysSpawn" "MultiplyWithRoot" null null)
    (`KismetSystemLibrary.K2_SetTimerDelegate` (delegate `ResetShot`) (`self.FireRate`))))

(event `ResetShot`
  (set `self.CanShoot` true))

(fn `UserConstructionScript`
  (`parent.UserConstructionScript`))