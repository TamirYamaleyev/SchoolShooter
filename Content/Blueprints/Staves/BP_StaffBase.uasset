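; BP_StaffBase is a base staff weapon that fires projectiles from its Arrow, with optional cone spread.
; StartFiring fires once or loops FireShot on a timer, gated by ammo, reload and cooldown; a blocked shot stops automatic fire.
; An empty staff reloads by converting the player's mana into ammo through ManaComponent, then waits ReloadTime.
; FireRate serves as shots per second for the loop but as seconds for the cooldown.
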(event `InitializeWeapon`
  (params (PlayerRef :type "/Game/Blueprints/Player/BP_Player Object Reference"))
  (bind _output_get (set `self.CachedPlayer` PlayerRef))
  (set `self.CachedManaComp` (`/Game/Blueprints/Player/BP_Player.Mana Component` _output_get)))

(event `self.ReceiveBeginPlay`
  (set `self.CurrentAmmo` (`self.MaxAmmo`)))

(fn `CheckCanFire`
  (returns (CanFire :type Boolean))
  (bind _hasammo (`self.HasAmmo`))
  (return (and _hasammo (not (`self.bIsReloading`)) (not (`self.bIsOnCooldown`)))))

(fn `ConsumeAmmo`
  (bind _result (`/Engine/EditorBlueprintResources/StandardMacros.DecrementInt` (`self.CurrentAmmo`))
    (:`  `
      (set `self.CurrentAmmo` _result))))

(fn `FireShot`
  (bind _canfire (`self.CheckCanFire`))
  (if _canfire
    (`self.ConsumeAmmo`)
    (`self.SpawnProjectile` (`self.ProjectileClass`))
    (set `self.bIsOnCooldown` true)
    (`KismetSystemLibrary.K2_SetTimer` null "ResetCooldown" (`self.FireRate`))
    (else
      (bind _hasammo (`self.HasAmmo`))
      (if (not _hasammo)
        (`self.ReloadStaff`))
      (if (`self.bIsAutomatic`)
        (`self.StopFiring`)))))

(fn `HasAmmo`
  (returns (HasAmmo :type Boolean))
  (return (> (`self.CurrentAmmo`) 0)))

(fn `ReloadStaff`
  (bind _cachedmanacomp (`self.CachedManaComp`))
  (`/Engine/EditorBlueprintResources/StandardMacros.IsValid` _cachedmanacomp
    (:`Is Valid`
      _)
    (:`Is Not Valid`
      (bind _asbp_player (cast `/Game/Blueprints/Player/BP_Player` (`GameplayStatics.GetPlayerPawn` 0)))
      (set `self.CachedManaComp` (`/Game/Blueprints/Player/BP_Player.Mana Component` _asbp_player))))
  (bind _ammounitstoreload (`/Game/Blueprints/Mana/BP_ManaComponent.TryConsumeMana` _cachedmanacomp (`self.MaxAmmo`) (`KismetMathLibrary.Conv_IntToDouble` (`self.ReloadCostPerUnit`))))
  (set `self.CurrentAmmo` _ammounitstoreload)
  (set `self.bIsReloading` true)
  (`KismetSystemLibrary.PrintString` "Reloading" true true (struct :`B` 1.0 :`A` 1.0))
  (`KismetSystemLibrary.K2_SetTimer` null "ResetCanFire" (`self.ReloadTime`)))

(fn `ResetCanFire`
  (set `self.bIsReloading` false)
  (`KismetSystemLibrary.PrintString` "Finished Reloading"))

(fn `ResetCooldown`
  (set `self.bIsOnCooldown` false))

(fn `SpawnProjectile`
  (params (ProjectileClass :type "/Game/Blueprints/Staves/Projectiles/BP_BaseProjectile Class Reference"))
  (bind _arrow (`self.Arrow`))
  (bind _returnvalue (`SceneComponent.K2_GetComponentToWorld` _arrow))
  (if (> (`self.Spread`) 0.0)
    (`|SpawnActorFromClass` ProjectileClass (`KismetMathLibrary.MakeTransform` (.location _returnvalue) (`KismetMathLibrary.MakeRotFromX` (`KismetMathLibrary.RandomUnitVectorInConeInDegrees` (`SceneComponent.GetForwardVector` _arrow) (`self.Spread`)))) "AdjustIfPossibleButAlwaysSpawn" "MultiplyWithRoot" null null)
    (else
      (`|SpawnActorFromClass` ProjectileClass (`KismetMathLibrary.MakeTransform` (.location _returnvalue) (`KismetMathLibrary.MakeRotator` (.roll (.rotation _returnvalue)) (.pitch (.rotation _returnvalue)) (.yaw (.rotation _returnvalue)))) "AdjustIfPossibleButAlwaysSpawn" "MultiplyWithRoot" null null))))

(fn `StartFiring`
  (if (`self.bIsAutomatic`)
    (bind _returnvalue (`KismetSystemLibrary.K2_SetTimer` null "FireShot" (/ 1.0 (`self.FireRate`)) true))
    (set `self.FireTimerHandle` _returnvalue)
    (else
      (`self.FireShot`))))

(fn `StopFiring`
  (`KismetSystemLibrary.K2_ClearAndInvalidateTimerHandle` (`self.FireTimerHandle`)))

(fn `UserConstructionScript`)