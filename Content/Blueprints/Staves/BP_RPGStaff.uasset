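; Base-style RPG staff weapon Blueprint that fires projectiles, limited by ammo and a cooldown.
; FireShot checks CheckCanFire, then consumes ammo, spawns the configured projectile class and starts a FireRate timer that calls ResetCooldown by name.
; When firing is blocked and the staff has no ammo, it calls ReloadStaff instead.
; The event graph holds only disabled default events.
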(fn `FireShot`
  (bind _canfire (`self.CheckCanFire`))
  (if _canfire
    (`self.ConsumeAmmo`)
    (`self.SpawnProjectile` (`self.ProjectileClass`))
    (set `self.bIsOnCooldown` true)
    (`KismetSystemLibrary.K2_SetTimer` null "ResetCooldown" (`self.FireRate`))
    (else
      (bind _hasammo (`self.HasAmmo`))
      (if (not _hasammo)
        (`self.ReloadStaff`)))))

(fn `UserConstructionScript`
  (`parent.UserConstructionScript`))