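; Fireball projectile actor from the staves set that explodes on impact.
; When its sphere component hits something, it calls DestroyActor, then applies full, non-falloff radial damage at the impact point within ExplosionRadius.
; A red debug sphere briefly draws the blast area, and the actor has no other active logic.
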(event `self.Sphere.OnComponentHit`
  (params (HitComponent :type "PrimitiveComponent Object Reference") (OtherActor :type "Actor Object Reference") (OtherComp :type "PrimitiveComponent Object Reference") (NormalImpulse :type "Vector Structure") (Hit :type "HitResult Structure (by ref)"))
  (bind (_bblockinghit _binitialoverlap _time _distance _location _impactpoint) (`GameplayStatics.BreakHitResult` Hit))
  (bind _explosionradius (`self.ExplosionRadius`))
  (`self.K2_DestroyActor`)
  (`KismetSystemLibrary.DrawDebugSphere` _impactpoint _explosionradius 12 (struct :`R` 1.0 :`A` 1.0) 1.0 10.0)
  (`GameplayStatics.ApplyRadialDamage` :`BaseDamage` (`self.Damage`) :`Origin` _impactpoint :`DamageRadius` _explosionradius :`DamageCauser` self :`InstigatedByController` null :`bDoFullDamage` true))

(fn `UserConstructionScript`
  (`parent.UserConstructionScript`))