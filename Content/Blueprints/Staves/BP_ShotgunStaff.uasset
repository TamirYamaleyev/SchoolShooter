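; Shotgun staff weapon Blueprint that fires either a single slug or a spread of birdshot pellets.
; FireShot calls CheckCanFire, then branches on IsSlugMode to spawn one slug projectile or loop over NumberOfPellets, applying SpreadBirdshot to each birdshot spawn.
; Only the slug branch sets a FireRate timer for ResetCanFire.
; The event graph holds only disabled default events.
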(fn `FireShot`
  (`self.CheckCanFire`)
  (if (`self.bIsSlugMode`)
    (`self.SpawnProjectile` (`self.ProjectileClass_Slug`))
    (`KismetSystemLibrary.K2_SetTimer` null "ResetCanFire" (`self.FireRate`))
    (else
      (for _ (range (`self.NumberOfPellets`))
        (set `self.Spread` (`self.Spread_Birdshot`))
        (`self.SpawnProjectile` (`self.ProjectileClass_Birdshot`))))))

(fn `UserConstructionScript`
  (`parent.UserConstructionScript`))