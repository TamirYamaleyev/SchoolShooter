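; BP_EnemyAIController is an enemy AI controller that starts the BT_Enemy behavior tree on BeginPlay.
; It first sets the TargetActor blackboard key to player character 0, so targeting does not depend on perception.
; The perception update event is empty; disconnected nodes for setting TargetActor from the sensed actor and CanSeePlayer from sensing success never run.
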(event `self.ReceiveBeginPlay`
  (`BlackboardComponent.SetValueAsObject` (`AIBlueprintHelperLibrary.GetBlackboard` null) "TargetActor" (`GameplayStatics.GetPlayerCharacter` 0))
  (`self.RunBehaviorTree` "/Game/Blueprints/Enemies/BT_Enemy.BT_Enemy"))

(event `self.AIPerception.OnTargetPerceptionUpdated`
  (params (Actor :type "Actor Object Reference") (Stimulus :type "AIStimulus Structure")))

(fn `UserConstructionScript`)