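; Enemy guard that patrols points, notices and chases the player, and reports its death to ShooterGameMode.
; An enum state machine dispatches through StateChanged, driven by AI Perception sight flags, timers and AIMoveTo.
; Reaching the player calls Lose on the game mode, while a give-up timer returns it to patrol.
; The attack state is unfinished: nothing sets it, and its in-range branch only delays.
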(event `Patrol`
  (`AIController.K2_SetFocus` (`AIBlueprintHelperLibrary.GetAIController` self) null)
  (`|AIMoveTo` self (0.0 0.0 0.0) (`|GetArrayItem` (`self.PatrolPoints`) (`self.PatrolIndex`)) 20.0
    (:`OnSuccess`
      (if (>= (`self.PatrolIndex`) (- (`KismetArrayLibrary.Array_Length` (`self.PatrolPoints`)) 1))
        (set `self.PatrolIndex` 0)
        (else
          (set `self.PatrolIndex` (+ (`self.PatrolIndex`) 1))))
      (`KismetSystemLibrary.Delay` 1.0)
      (`self.Patrol`))))

(event `self.ReceiveBeginPlay`
  (bind _asbp_player (cast `/Game/Blueprints/Player/BP_Player` (`GameplayStatics.GetPlayerCharacter` 0)))
  (set `self.PlayerRef` _asbp_player)
  (`KismetSystemLibrary.PrintString` "Player Ref Saved" true true (struct :`G` 1.0 :`A` 1.0) 2.0 "playerfound")
  (set `self.AttackRange` (`KismetMathLibrary.RandomFloatInRange` (`self.MinAttackRange`) (`self.MaxAttackRange`)))
  (set `self.CurrentState` "NewEnumerator0")
  (`self.StateChanged`))

(event `self.AIPerception.OnTargetPerceptionUpdated`
  (params (Actor :type "Actor Object Reference") (Stimulus :type "AIStimulus Structure"))
  (if (== Actor (`self.PlayerRef`))
    (if (`.bSuccessfullySensed` (break `AIStimulus` Stimulus))
      (if (not (`self.IsFollowing`))
        (set `self.IsSeeingPlayer` true)
        (set `self.CurrentState` "NewEnumerator1")
        (`self.StateChanged`))
      (else
        (set `self.IsSeeingPlayer` false)))))

(event `NoticePlayer`
  (bind _playerref (`self.PlayerRef`))
  (`Controller.StopMovement` (`AIBlueprintHelperLibrary.GetAIController` self))
  (`/Engine/EditorBlueprintResources/StandardMacros.IsValid` _playerref
    (:`Is Valid`
      (`AIController.K2_SetFocus` (`AIBlueprintHelperLibrary.GetAIController` self) _playerref)
      (`KismetSystemLibrary.K2_SetTimerDelegate` (delegate `EndNotice`) (`self.NoticeTimer`)))
    (:`Is Not Valid`
      (`KismetSystemLibrary.PrintString` "Invalid Player Ref!"))))

(event `EndNotice`
  (if (`self.IsSeeingPlayer`)
    (set `self.CurrentState` "NewEnumerator2")
    (else
      (set `self.CurrentState` "NewEnumerator0")))
  (`self.StateChanged`))

(event `FollowPlayer`
  (set `self.IsFollowing` true)
  (`|AIMoveTo` self (0.0 0.0 0.0) (`self.PlayerRef`) 100.0
    (:`then`
      (`KismetSystemLibrary.K2_SetTimerDelegate` (delegate `GiveUp`) (`self.GiveUpTimer`)))
    (:`OnSuccess`
      (bind _asshooter_game_mode (cast `/Game/ShooterGameMode` (`GameplayStatics.GetGameMode`)))
      (`/Game/ShooterGameMode.Lose` _asshooter_game_mode))))

(event `GiveUp`
  (set `self.CurrentState` "NewEnumerator0")
  (`self.StateChanged`))

(event `StateChanged`
  (switch `/Game/Enums/E_GuardState` (`self.CurrentState`)
    (:`NewEnumerator0`
      (`self.Patrol`))
    (:`NewEnumerator1`
      (`self.NoticePlayer`))
    (:`NewEnumerator2`
      (`self.FollowPlayer`))
    (:`NewEnumerator3`
      (`self.AttackPlayer`))))

(event `self.ReceiveTick`
  (params (DeltaSeconds :type "Float (single-precision)"))
  (`KismetSystemLibrary.PrintString` (`|GetEnumeratorNameAsString` (`self.CurrentState`)) true true (struct :`G` 0.66 :`B` 1.0 :`A` 1.0) 2.0 "State"))

(event `self.ReceiveAnyDamage`
  (params (Damage :type "Float (single-precision)") (DamageType :type "DamageType Object Reference") (InstigatedBy :type "Controller Object Reference") (DamageCauser :type "Actor Object Reference"))
  (bind _health (`self.Health`))
  (set `self.Health` (- (`self.Health`) Damage))
  (`KismetSystemLibrary.PrintString` (`KismetStringLibrary.Conv_DoubleToString` _health) true true (struct :`G` 1.0 :`A` 1.0) 5.0 "Health")
  (if (<= _health 0.0)
    (bind _asshooter_game_mode (cast `/Game/ShooterGameMode` (`GameplayStatics.GetGameMode`)))
    (`/Game/ShooterGameMode.GuardKilled` _asshooter_game_mode)
    (`self.K2_DestroyActor`)))

(event `AttackPlayer`
  (bind _returnvalue (`AIBlueprintHelperLibrary.GetAIController` self))
  (if (`KismetSystemLibrary.IsValid` (`self.PlayerRef`))
    (`Controller.StopMovement` _returnvalue)
    (`AIController.K2_SetFocus` _returnvalue (`self.PlayerRef`))
    (if (`self.IsSeeingPlayer`)
      (if (> (`self.GetDistanceTo` (`self.PlayerRef`)) (`self.AttackRange`))
        (set `self.CurrentState` "NewEnumerator2")
        (`self.StateChanged`)
        (else
          (`KismetSystemLibrary.Delay` 0.2)
          (if true
            _)))
      (else
        (set `self.CurrentState` "NewEnumerator0")
        (`self.StateChanged`)))
    (else
      (set `self.CurrentState` "NewEnumerator0")
      (`self.StateChanged`))))

(fn `UserConstructionScript`)