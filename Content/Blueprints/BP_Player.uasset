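; Player character Blueprint handling camera-relative WASD movement, mouse look, jumping and a switchable weapon inventory.
; Raw key events set movement axes applied each Tick, while Enhanced Input drives firing and weapon cycling after BeginPlay loads IMC_Default.
; SpawnWeapon attaches new weapons to the mesh's rifle socket, and switching toggles their visibility.
; CheckPickupCollision sphere-traces for BPI_Interaction actors to message, but its looping timer is unconnected.
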(event `InputVectorAxis|Mouse2D`
  (params (AxisValue :type "Vector Structure"))
  ; Camera + Movement
  (`self.AddControllerYawInput` AxisValue_X)
  (`self.AddControllerPitchInput` (* AxisValue_Y -1.0)))

(event `Key|W`
  (params (Key :type "Key Structure"))
  ; Camera + Movement
  (:`Pressed`
    (set `self.WDown` true)
    (set `self.ForwardAxis` (+ (`KismetMathLibrary.Conv_BoolToDouble` (`self.WDown`)) (* (`KismetMathLibrary.Conv_BoolToDouble` (`self.SDown`)) -1.0)) :!label _label))
  (:`Released`
    (set `self.WDown` false)
    (goto _label)))

(event `Key|S`
  (params (Key :type "Key Structure"))
  ; Camera + Movement
  (:`Pressed`
    (set `self.SDown` true)
    (goto _label))
  (:`Released`
    (set `self.SDown` false)
    (goto _label)))

(event `Key|D`
  (params (Key :type "Key Structure"))
  ; Camera + Movement
  (:`Pressed`
    (set `self.DDown` true)
    (set `self.RightAxis` (+ (`KismetMathLibrary.Conv_BoolToDouble` (`self.DDown`)) (* (`KismetMathLibrary.Conv_BoolToDouble` (`self.ADown`)) -1.0)) :!label _label_2))
  (:`Released`
    (set `self.DDown` false)
    (goto _label_2)))

(event `Key|A`
  (params (Key :type "Key Structure"))
  ; Camera + Movement
  (:`Pressed`
    (set `self.ADown` true)
    (goto _label_2))
  (:`Released`
    (set `self.ADown` false)
    (goto _label_2)))

(event `self.ReceiveTick`
  (params (DeltaSeconds :type "Float (single-precision)"))
  (bind _camera (`self.Camera`))
  (bind (_returnvalue_x _returnvalue_y) (`KismetMathLibrary.BreakVector` (`SceneComponent.GetForwardVector` _camera)))
  ; Camera + Movement
  (`self.AddMovementInput` (+ (`KismetMathLibrary.Normal` (* (`KismetMathLibrary.MakeVector` _returnvalue_x _returnvalue_y) (`self.ForwardAxis`))) (* (`SceneComponent.GetRightVector` _camera) (`self.RightAxis`)))))

(event `Key|SpaceBar`
  (params (Key :type "Key Structure"))
  ; Camera + Movement
  (:`Pressed`
    (`self.Jump`)))

(event `self.ReceiveBeginPlay`
  (bind _returnvalue (subsystem `EnhancedInputLocalPlayerSubsystem`))
  (`EnhancedInputSubsystemInterface.ClearAllMappings` _returnvalue)
  (`EnhancedInputSubsystemInterface.AddMappingContext` _returnvalue "/Game/Input/IMC_Default.IMC_Default" 0 (struct)))

(event `EnhancedInput|/Game/Input/Actions/IA_Shoot`
  (params (ActionValue :type Boolean) (ElapsedSeconds :type "Float (double-precision)") (TriggeredSeconds :type "Float (double-precision)") (InputAction :type "InputAction Object Reference" :default "/Game/Input/Actions/IA_Shoot.IA_Shoot"))
  (:`Started`
    (`/Engine/EditorBlueprintResources/StandardMacros.IsValid` (`self.CurrentWeapon`)
      (:`Is Valid`
        (`/Game/Blueprints/Staves/BP_StaffBase.StartFiring` (`self.CurrentWeapon`))))))

(event `EnhancedInput|/Game/Input/Actions/IA_SwitchWeapon`
  (params (ActionValue :type Boolean) (ElapsedSeconds :type "Float (double-precision)") (TriggeredSeconds :type "Float (double-precision)") (InputAction :type "InputAction Object Reference" :default "/Game/Input/Actions/IA_SwitchWeapon.IA_SwitchWeapon"))
  (:`Started`
    (if (`KismetArrayLibrary.Array_IsNotEmpty` (`self.Weapons`))
      (set `self.CurrentWeapon` (`|GetArrayItem` (`self.Weapons`) (mod (+ (`KismetArrayLibrary.Array_Find` (`self.Weapons`) (`self.CurrentWeapon`)) 1) (`KismetArrayLibrary.Array_Length` (`self.Weapons`)))))
      (for _array_element (`self.Weapons`)
        (if (!= _array_element (`self.CurrentWeapon`))
          (`SceneComponent.SetVisibility` (`Actor.RootComponent` _array_element) false true)
          (`SceneComponent.SetVisibility` (`Actor.RootComponent` (`self.CurrentWeapon`)) true true))))))

(event `CheckPickupCollision`
  (bind _returnvalue (`self.K2_GetActorLocation`))
  (bind (_outhits _returnvalue_2) (`KismetSystemLibrary.SphereTraceMultiForObjects` _returnvalue _returnvalue 150.0 (`|MakeArray` "ObjectTypeQuery4" :!type "EObjectTypeQuery Enum")))
  (if _returnvalue_2
    (for _array_element _outhits
      (bind (_bblockinghit _binitialoverlap _time _distance _location _impactpoint _normal _impactnormal _physmat _hitactor) (`GameplayStatics.BreakHitResult` _array_element))
      (if (`KismetSystemLibrary.DoesImplementInterface` _hitactor "/Game/Blueprints/Interfaces/BPI_Interaction.BPI_Interaction_C")
        (message `/Game/Blueprints/Interfaces/BPI_Interaction.Interact` _hitactor self)))))

(event `SpawnWeapon`
  (params (Weapon :type "/Game/Blueprints/Staves/BP_StaffBase Class Reference"))
  (bind _currentweapon (`self.CurrentWeapon`))
  (`/Engine/EditorBlueprintResources/StandardMacros.IsValid` _currentweapon
    (:`Is Valid`
      (`SceneComponent.SetVisibility` (`Actor.RootComponent` _currentweapon) false true))
    (:`Is Not Valid`
      _))
  (bind _returnvalue (`|SpawnActorFromClass` Weapon (`self.GetTransform`) "AlwaysSpawn" "MultiplyWithRoot" null null))
  (bind _output_get (set `self.CurrentWeapon` _returnvalue))
  (`self.K2_AttachToComponent` _output_get (`self.Mesh`) "Rifle_Socket" "SnapToTarget" "SnapToTarget" "SnapToTarget" true)
  (`KismetArrayLibrary.Array_Add` (`self.Weapons`) (`self.CurrentWeapon`)))

(fn `UserConstructionScript`)